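; Game mode for an infinite terrain game that spawns BP_Tile actors end to end and keeps a score of conquered tiles.
; BeginPlay fills a nav mesh volume pool, then loops over a few tile spawns with a delayed score increment.
; Each tile receives the shared pool and supplies the attach transform for the next one.
; Scoring also fetches the HUD widget but does not use it.
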(event EventBeginPlay
  (Class|InfiniteTerrainGameMode|PopulateVolumeBoundsPool)
  (for _index (range 0 3)
    (CallFunction|SpawnTIle)
    (Utilities|FlowControl|Delay 2.0)
    (CallFunction|NewTileConquered)))

(fn ConstructionScript)

(fn SpawnTIle
  (bind _returnvalue (Game|SpawnActorfromClass "/Game/Dynamic/Terrain/BP_Tile.BP_Tile_C" (Variables|Default|GetNextTileTransform) "Undefined" 0 0))
  (Class|Tile|SetNavVolumeActorPool _returnvalue (Variables|Default|GetNavMeshVolumeActorPool))
  (bind _attachtransform (Default|GetAttachLocation _returnvalue))
  (Variables|Default|SetNextTileTransform _attachtransform))

(fn NewTileConquered
  (Variables|Default|SetScore (+ (Variables|Default|GetScore) 1))
  (bind _asbp_hud (Utilities|Casting|CastToBP_HUD (HUD|GetHUD (Game|GetPlayerController 0))))
  (bind _hudwidget (Default|GetHudWidget _asbp_hud)))

(fn GetScore
  (return (Variables|Default|GetScore)))