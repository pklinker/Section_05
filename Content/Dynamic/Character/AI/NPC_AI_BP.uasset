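; AI controller for guard NPCs that patrol and target the player through AI perception.
; On BeginPlay it initializes the PatrolData blackboard and runs the GuardBehavior tree.
; Perception updates set EnemyKey to a sensed actor whose instigator is player-controlled, and clear it when any stimulus is not successfully sensed.
; An unconnected older chain stores a fixed player location instead, and FindPatrolRoute is an empty stub.
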(event OnTargetPerceptionUpdated(AIPerception)
  (params (Actor :type Actor%20Object%20Reference) (Stimulus :type AI%20Stimulus%20Structure))
  (CallFunction|UpdateBlackboardEnemyKey Actor Stimulus Actor))

(event EventBeginPlay
  ;[1 1 1] THis will get the robot to point their gun at the player as the player moves.
  (bind _blackboardcomponent (Class|AIController|UseBlackboard "/Game/Dynamic/Character/AI/PatrolData.PatrolData"))
  (AI|RunBehaviorTree "/Game/Dynamic/Character/AI/GuardBehavior.GuardBehavior")
  (Variables|Default|SetBlackboardComp _blackboardcomponent))

(fn ConstructionScript)

(fn FindPatrolRoute
  (params (Blackboard :type Blackboard%20Component%20Object%20Reference)))

(fn UpdateBlackboardEnemyKey
  (params (ObjectValue :type Object%20Object%20Reference) (AIStimulus :type AI%20Stimulus%20Structure%20%28by%20ref%29) (self2 :type Actor%20Object%20Reference))
  (bind _enemykey (Variables|Default|GetEnemyKey))
  (bind _blackboard (Variables|Default|GetBlackboard))
  (if (.bSuccessfullySensed (Utilities|Struct|BreakAIStimulus AIStimulus))
    ;[1 1 1] Make sure the pawn seen is the player
    (if (Pawn|IsPlayerControlled (Variables|/Script/Engine.Actor|GetInstigator self2))
      (AI|Components|Blackboard|SetValueasObject _blackboard _enemykey ObjectValue))
    (else
      (AI|Components|Blackboard|ClearValue _blackboard _enemykey))))