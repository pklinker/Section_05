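; Behavior tree task that makes an AI-controlled BP_Character aim and shoot at the player.
; On execute it turns on the character's aiming and shooting behavior flags and sets the controller's focus to the blackboard Target actor.
; It never finishes execution itself, so it stays active until aborted, when it clears both flags and the focus and then finishes the abort.
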(event EventReceiveExecuteAI
  (params (OwnerController :type AI%20Controller%20Object%20Reference) (ControlledPawn :type Pawn%20Object%20Reference))
  ;[1 1 1] Enable aiming and shooting by the NPCs.
  (bind _asbp_character (Utilities|Casting|CastToBP_Character ControlledPawn))
  (bind _output_get (Variables|/Game/Dynamic/Character/Behavior/BP_Character.BP_Character_C|SetAImingBehavior _asbp_character true))
  (Variables|/Game/Dynamic/Character/Behavior/BP_Character.BP_Character_C|SetShootingBehavior _asbp_character _output_get)
  ;[1 1 1] Set the focus to the player
  (AI|SetFocus OwnerController (AI|BehaviorTree|GetBlackboardValueasActor (Variables|Default|GetTarget))))

(event EventReceiveAbortAI
  (params (OwnerController :type AI%20Controller%20Object%20Reference) (ControlledPawn :type Pawn%20Object%20Reference))
  ;[1 1 1] When AI aborts, turn off shooting and turn off aiming.
  (bind _asbp_character (Utilities|Casting|CastToBP_Character ControlledPawn))
  (Variables|/Game/Dynamic/Character/Behavior/BP_Character.BP_Character_C|SetAImingBehavior _asbp_character false)
  (Variables|/Game/Dynamic/Character/Behavior/BP_Character.BP_Character_C|SetShootingBehavior _asbp_character false)
  ;[1 1 1] No longer focus on player
  (AI|ClearFocus OwnerController)
  (Class|BTTaskBlueprintBase|FinishAbort))