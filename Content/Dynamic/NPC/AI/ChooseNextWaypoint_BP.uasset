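; Behavior tree task that picks the next patrol waypoint for an AI-controlled NPC.
; It writes the patrol point at the Blackboard Index to the Waypoint key, then advances Index with wraparound and finishes successfully.
; GetPatrolPoints is meant to supply the points from the controlled pawn, but its entry does nothing and its return logic is unconnected.
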(event EventReceiveExecuteAI
  (params (OwnerController :type AI%20Controller%20Object%20Reference) (ControlledPawn :type Pawn%20Object%20Reference))
  (bind _output_get (CallFunction|GetPatrolPoints ControlledPawn))
  (bind _index (CallFunction|SetNextWaypoint _output_get))
  (CallFunction|CycleWaypointIndex _index)
  (AI|BehaviorTree|FinishExecute true))

(fn GetPatrolPoints
  (params (Object :type Object%20Object%20Reference)))

(fn SetNextWaypoint
  (params (Array :type Array%20of%20Actor%20Object%20References))
  (bind _index (Variables|Default|GetIndex))
  (bind _returnvalue (Class|BTFunctionLibrary|GetBlackboardValueasInt _index))
  (Class|BTFunctionLibrary|SetBlackboardValueasObject (Variables|Default|GetWaypoint) (Utilities|Array|Get(acopy) Array _returnvalue))
  (return _returnvalue))

(fn CycleWaypointIndex
  (params (A :type Integer))
  (Class|BTFunctionLibrary|SetBlackboardValueasInt (Variables|Default|GetIndex) (Math|Integer|%(Integer) (+ A 1) (Utilities|Array|Length (Variables|Default|GetPatrol%20Points)))))