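; AI controller for guard NPCs that detects the player and has the controlled character aim its weapon.
; On BeginPlay it loads the PatrolData blackboard and runs the GuardBehavior tree.
; AI perception stores a sensed player-controlled actor under EnemyKey and clears the key when a stimulus is lost.
; Tick sets the character's aiming flag from whether a focus actor exists; FindPatrolRoute is an empty stub.
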(event OnTargetPerceptionUpdated(AIPerception)
  (params (Actor :type Actor%20Object%20Reference) (Stimulus :type AI%20Stimulus%20Structure))
  (bind _enemykey (Variables|Default|GetEnemyKey))
  (bind _blackboard (Variables|Default|GetBlackboard))
  (if (.bSuccessfullySensed (Utilities|Struct|BreakAIStimulus Stimulus))
    ;[1 1 1] Make sure the pawn seen is the player
    (if (Pawn|IsPlayerControlled (Variables|/Script/Engine.Actor|GetInstigator Actor))
      (AI|Components|Blackboard|SetValueasObject _blackboard _enemykey Actor))
    (else
      (AI|Components|Blackboard|ClearValue _blackboard _enemykey))))

(event EventBeginPlay
  ;[1 1 1] THis will get the robot to point their gun at the player as the player moves.
  (bind _blackboardcomponent (Class|AIController|UseBlackboard "/Game/Dynamic/NPC/AI/PatrolData.PatrolData"))
  (AI|RunBehaviorTree "/Game/Dynamic/NPC/AI/GuardBehavior.GuardBehavior")
  (Variables|Default|SetBlackboardComp _blackboardcomponent))

(event EventTick
  (params (DeltaSeconds :type Float%20%28single-precision%29))
  ;[1 1 1] Sets aiming if they NPC finds the player - has focus
  (bind _asue_4asp_character (Utilities|Casting|CastToUe4ASP_Character (Pawn|GetControlledPawn)))
  (Variables|/Game/Dynamic/NPC/Behavior/Ue4ASP_Character.Ue4ASP_Character_C|SetAIming _asue_4asp_character (Utilities|IsValid (Class|AIController|GetFocusActor))))

(fn ConstructionScript)

(fn FindPatrolRoute
  (params (Blackboard :type Blackboard%20Component%20Object%20Reference)))