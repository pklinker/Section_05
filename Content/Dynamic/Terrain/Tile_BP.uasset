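; Terrain tile for an infinite world, with a barrier wall that opens for the player and seals behind them.
; Overlapping OpenBarrierBox disables the wall's collision and turns it green; leaving restores collision, turns it red and asks InfiniteTerrainGameMode to spawn another tile.
; Leaving DestroyTileBox destroys this tile.
; GetAttachLocation exposes the Arrow's world transform as the attach point.
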(event OnComponentEndOverlap(DestroyTileBox)
  (params (OverlappedComponent :type Primitive%20Component%20Object%20Reference) (OtherActor :type Actor%20Object%20Reference) (OtherComp :type Primitive%20Component%20Object%20Reference) (OtherBodyIndex :type Integer))
  ;[1 1 1] Destroy previous tile when player leaves destroy tile box.
  (Utilities|IsPlayerActor OtherActor)
  (Actor|DestroyActor))

(event OnComponentBeginOverlap(OpenBarrierBox)
  (params (OverlappedComponent :type Primitive%20Component%20Object%20Reference) (OtherActor :type Actor%20Object%20Reference) (OtherComp :type Primitive%20Component%20Object%20Reference) (OtherBodyIndex :type Integer) (bFromSweep :type Boolean) (SweepResult :type Hit%20Result%20Structure%20%28by%20ref%29))
  ;[1 1 1] Unlock walls at start.
  (Utilities|IsPlayerActor OtherActor)
  (CallFunction|UnlockWall))

(event OnComponentEndOverlap(OpenBarrierBox)
  (params (OverlappedComponent :type Primitive%20Component%20Object%20Reference) (OtherActor :type Actor%20Object%20Reference) (OtherComp :type Primitive%20Component%20Object%20Reference) (OtherBodyIndex :type Integer))
  ;[1 1 1] When the player goes through a wall and triggers the box collision, lock the wall.
  (Utilities|IsPlayerActor OtherActor)
  (CallFunction|LockWall)
  ;[1 1 1] Spawn a new tile at the end of the line to make an infinite world.
  (bind _asinfinite_terrain_game_mode (Utilities|Casting|CastToInfiniteTerrainGameMode (Game|GetGameMode)))
  (Default|SpawnTIle _asinfinite_terrain_game_mode))

(event Collision|EventActorBeginOverlap
  (params (OtherActor :type Actor%20Object%20Reference)))

(event EventTick
  (params (DeltaSeconds :type Float%20%28single-precision%29)))

(fn ConstructionScript)

(fn GetAttachLocation
  (return (Transformation|GetWorldTransform (Variables|Default|GetArrow))))

(fn UnlockWall
  (Collision|SetCollisionEnabled (Variables|Default|GetBarrierWall) "NoCollision")
  (Rendering|Material|SetMaterial (Variables|Default|GetBarrierWall) 0 "/Game/Dynamic/Terrain/GreenBarrier.GreenBarrier"))

(fn LockWall
  (Collision|SetCollisionEnabled (Variables|Default|GetBarrierWall) "QueryAndPhysics")
  (Rendering|Material|SetMaterial (Variables|Default|GetBarrierWall) 0 "/Game/Dynamic/Terrain/RedBarrier.RedBarrier"))